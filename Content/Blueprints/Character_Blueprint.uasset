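; Player character that walks, jumps and climbs across walls with camera-relative input, using Flying movement mode as the grab state.
; Pushing into a wall found by a forward trace builds GrabIntent until the character latches on.
; While grabbed, input is projected onto the surface plane and CheckEdges traces for inner and outer corners.
; Turn sets targets for a timeline that blends onto each new surface, restoring Walking on upward-facing ones.
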(event `InputAction|Jump`
  (params (Key :type "Key Structure"))
  (:`Pressed`
    (`self.Jump`)))

(event `self.ReceiveTick`
  (params (DeltaSeconds :type "Float (single-precision)"))
  (bind (_returnvalue_roll _returnvalue_pitch _returnvalue_yaw) (`KismetMathLibrary.BreakRotator` (`self.K2_GetActorRotation`)))
  (bind _returnvalue (`self.K2_GetActorLocation`))
  (bind _targetnormal (`self.TargetNormal`))
  (bind _charactermovement (`self.CharacterMovement`))
  (bind _grabtostanding (`self.GrabToStanding`))
  (bind _returnvalue_2 (`KismetMathLibrary.TransformDirection` (`SceneComponent.K2_GetComponentToWorld` (`self.Camera`)) (`KismetMathLibrary.MakeVector` (`self.GetInputAxisValue`) (`self.GetInputAxisValue`))))
  (bind _returnvalue_3 (`KismetMathLibrary.ProjectVectorOnToPlane` (`KismetMathLibrary.TransformDirection` (`SceneComponent.K2_GetComponentToWorld` (`self.Camera`)) (`KismetMathLibrary.MakeVector` 0.0 (`self.GetInputAxisValue`) (`self.GetInputAxisValue`))) (`self.TargetNormal`)))
  (switch `EMovementMode` (`CharacterMovementComponent.MovementMode` (`self.CharacterMovement`))
    (:`MOVE_Walking`
      ;[1 1 1] Walk/Fall movement
      ;;[1 1 1] Common movement
      (`self.AddMovementInput` _returnvalue_2 :!label _label)
      (`self.K2_SetActorRotation` (`KismetMathLibrary.MakeRotator` 0.0 0.0 _returnvalue_yaw))
      (`CapsuleComponent.SetCapsuleHalfHeight` (`self.CapsuleComponent`) (`self.StandingHalfHeight`) true)
      (set `CharacterMovementComponent.RotationRate` (select `bool` (`NavMovementComponent.IsFalling` _charactermovement) :`false` (`self.RotationSpeedGround`) :`true` (`self.RotationSpeedAir`)) _charactermovement)
      (`SceneComponent.K2_SetRelativeRotation` :`self` (`self.SpringArm`))
      (set `CharacterMovementComponent.bOrientRotationToMovement` true (`self.CharacterMovement`))
      ;;[1 1 1] Checks if player is forcing towards a wall
      (bind _outhit (`KismetSystemLibrary.LineTraceSingle` :`Start` _returnvalue :`End` (+ _returnvalue (* (`self.GetActorForwardVector`) 68.0)) :`TraceChannel` "TraceTypeQuery1" :`DrawDebugType` "ForOneFrame"))
      (bind (_bblockinghit _binitialoverlap _time _distance _location _impactpoint _normal) (`GameplayStatics.BreakHitResult` _outhit))
      (if (and (> (`KismetMathLibrary.Dot_VectorVector` _returnvalue_2 (`KismetMathLibrary.NegateVector` _normal)) 0.5) _bblockinghit)
        (set `self.GrabIntent` (+ (`self.GrabIntent`) 0.05))
        (else
          (set `self.GrabIntent` 0.0)))
      (if (> (`self.GrabIntent`) 1.0)
        (`CharacterMovementComponent.SetMovementMode` (`self.CharacterMovement`) "MOVE_Flying" 0)
        (`self.Turn` _normal _location (`KismetMathLibrary.MakeRotFromXZ` (0.0 0.0 1.0) _normal))))
    (:`MOVE_Falling`
      (goto _label))
    (:`MOVE_Flying`
      ;[1 1 1] Grab movement
      (`CapsuleComponent.SetCapsuleHalfHeight` (`self.CapsuleComponent`) 0.0 true)
      (`SceneComponent.K2_SetRelativeRotation` (`self.SpringArm`) (struct :`Pitch` -90.0) false false)
      (set `CharacterMovementComponent.bOrientRotationToMovement` false (`self.CharacterMovement`))
      (if (`self.Aligned`)
        ;;[1 1 1] Moves parallel to the wall
        (`self.AddMovementInput` _returnvalue_3)
        (if (> (`KismetMathLibrary.VSize` _returnvalue_3) 0.0)
          ;;[1 1 1] Rotate towards desired input direction
          (`self.K2_SetActorRotation` (`KismetMathLibrary.RLerp` (`self.K2_GetActorRotation`) (`KismetMathLibrary.MakeRotFromXZ` _returnvalue_3 (`self.TargetNormal`)) 0.1 true))
          (bind (_returnvalue_4 _location_2 _normal_2) (`self.CheckEdges`))
          (if _returnvalue_4
            ;;[1 1 1] Turn a corner
            (`self.Turn` _normal_2 _location_2 (`KismetMathLibrary.ComposeRotators` (`self.K2_GetActorRotation`) (`KismetMathLibrary.RotatorFromAxisAndAngle` (`KismetMathLibrary.Normal` (`KismetMathLibrary.Cross_VectorVector` _targetnormal _normal_2)) (`KismetMathLibrary.RadiansToDegrees` (`KismetMathLibrary.Acos` (`KismetMathLibrary.FClamp` (`KismetMathLibrary.Dot_VectorVector` _targetnormal _normal_2) -1.0))))))))
        (else
          ;;[1 1 1] Smooth rotate to target
          (bind (_direction _newtrack_1) (`Timeline|RotateToNormal`)
            (:`Update`
              (`self.K2_SetActorRotation` (`KismetMathLibrary.RLerp` (`self.SourceRotation`) (`self.TargetRotation`) _newtrack_1 true))
              (`self.K2_SetActorLocation` (`KismetMathLibrary.VLerp` (`self.SourcePosition`) (`self.TargetPosition`) _newtrack_1)))
            (:`Finished`
              ;;[1 1 1] Grab to standing
              (set `self.Aligned` (not _grabtostanding))
              (if _grabtostanding
                (`CharacterMovementComponent.SetMovementMode` (`self.CharacterMovement`) "MOVE_Walking" 0)))))))))

(fn `CheckEdges`
  (returns (ReturnValue :type Boolean) (Location :type "Vector Structure") (Normal :type "Vector Structure"))
  (bind _returnvalue (`self.K2_GetActorLocation`))
  (bind _returnvalue_2 (* (`self.GetActorUpVector`) -68.0))
  ;[1 1 1] Check inner corners
  (bind _outhit (`KismetSystemLibrary.LineTraceSingle` :`Start` (+ (`self.K2_GetActorLocation`) (* (`KismetMathLibrary.Normal` (`MovementComponent.Velocity` (`self.CharacterMovement`))) 80.0) _returnvalue_2) :`End` (+ (`self.K2_GetActorLocation`) _returnvalue_2) :`TraceChannel` "TraceTypeQuery1" :`DrawDebugType` "ForDuration"))
  (bind (_bblockinghit _binitialoverlap _time _distance _location _impactpoint _normal) (`GameplayStatics.BreakHitResult` _outhit))
  (bind _returnvalue_3 (and _bblockinghit (not _binitialoverlap)))
  (if _returnvalue_3
    (return _returnvalue_3 _location _normal)
    (else
      ;[1 1 1] Check outer corners
      (bind _outhit_2 (`KismetSystemLibrary.LineTraceSingle` :`Start` _returnvalue :`End` (+ _returnvalue (* (`KismetMathLibrary.Normal` (`MovementComponent.Velocity` (`self.CharacterMovement`))) 80.0)) :`TraceChannel` "TraceTypeQuery1" :`DrawDebugType` "ForDuration" :`TraceColor` (struct :`G` 0.159694 :`B` 1.0 :`A` 1.0) :`TraceHitColor` (struct :`R` 1.0 :`G` 0.905883 :`A` 1.0)))
      (bind (_bblockinghit_2 _binitialoverlap_2 _time_2 _distance_2 _location_2 _impactpoint_2 _normal_2) (`GameplayStatics.BreakHitResult` _outhit_2))
      (return (and _bblockinghit_2 (not _binitialoverlap_2)) _location_2 _normal_2))))

(fn `Turn`
  (params (TargetNormal :type "Vector Structure") (TargetPosition :type "Vector Structure") (TargetRotation :type "Rotator Structure"))
  (bind _returnvalue (> (`KismetMathLibrary.Dot_VectorVector` TargetNormal (0.0 0.0 1.0)) 0.5))
  (set `self.TargetNormal` TargetNormal)
  (set `self.TargetPosition` (+ TargetPosition (* TargetNormal (select `bool` _returnvalue :`false` 34.0 :`true` 100.0))))
  (set `self.SourceRotation` (`self.K2_GetActorRotation`))
  (set `self.SourcePosition` (`self.K2_GetActorLocation`))
  (set `self.TargetRotation` TargetRotation)
  (set `self.Aligned` false)
  (set `self.GrabToStanding` _returnvalue)
  (`TimelineComponent.SetPlaybackPosition` (`self.RotateToNormal`) 0.0 false false))

(fn `UserConstructionScript`)